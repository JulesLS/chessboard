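; Chess piece actor that reports itself to the chess controller as the hovered piece and, when clicked, highlights its possible moves.
; Only Rook moves are implemented, scanning the game instance's chessboard in four directions up to and including the first occupied tile, regardless of owner.
; Descending scans loop over negated indices and apply Abs.
; Found tiles accumulate in PossibleTiles, which is never cleared here, and get their material swapped.
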(event OnBeginCursorOver(pieceMesh)
  (params (TouchedComponent :type Primitive%20Component%20Object%20Reference))
  (Variables|/Game/Blueprint/BP_ChessController.BP_ChessController_C|SethoveredPiece (CallFunction|GetChessController1) self))

(event OnEndCursorOver(pieceMesh)
  (params (TouchedComponent :type Primitive%20Component%20Object%20Reference))
  (Variables|/Game/Blueprint/BP_ChessController.BP_ChessController_C|SethoveredPiece (CallFunction|GetChessController1) 0))

(event OnClicked(pieceMesh)
  (params (TouchedComponent :type Primitive%20Component%20Object%20Reference) (ButtonPressed :type Key%20Structure :default "None"))
  (CallFunction|CalculatePossibleMoves))

(event Custom|calculatePossibleMoves
  (switch Utilities|FlowControl|Switch|SwitchonE_PieceType (Variables|Default|GetpieceType)
    (:NewEnumerator1
      (CallFunction|CalculateRooksMoves)
      (CallFunction|DisplayPossibleMoves))))

(event Custom|displayPossibleMoves
  (for _array_element (Variables|Default|GetpossibleTiles)
    (Rendering|Material|SetMaterial (Variables|/Game/Blueprint/BP_ChessTile.BP_ChessTile_C|GettileMesh _array_element) 0 "/Game/Blueprint/Materials/M_Echiquier.M_Echiquier")))

(fn ConstructionScript)

(fn CalculateRooksMoves
  (bind _currenttile (Variables|Default|GetcurrentTile))
  (bind _currenttile_2 (Variables|Default|GetcurrentTile))
  (bind _currenttile_3 (Variables|Default|GetcurrentTile))
  (bind _currenttile_4 (Variables|Default|GetcurrentTile))
  (bind _tilerow (Variables|/Game/Blueprint/BP_ChessTile.BP_ChessTile_C|GettileRow _currenttile_3))
  (bind _tilerow_2 (Variables|/Game/Blueprint/BP_ChessTile.BP_ChessTile_C|GettileRow _currenttile_4))
  (bind _tilecolumn (Variables|/Game/Blueprint/BP_ChessTile.BP_ChessTile_C|GettileColumn _currenttile))
  (bind _tilecolumn_2 (Variables|/Game/Blueprint/BP_ChessTile.BP_ChessTile_C|GettileColumn _currenttile_2))
  (bind _column (CallFunction|SelectonName _tilecolumn_2))
  (bind _column_2 (CallFunction|SelectonName _tilecolumn))
  ;[0 0 0 1 36] Calculate Vertical Moves
  (bind _index (Utilities|FlowControl|ForLoopwithBreak (Math|Integer|Clamp(Integer) (+ _tilerow 1) 1 8) (Math|Integer|Clamp(Integer) (+ _tilerow 8) 1 8) :!label _label)
    (:LoopBody
      (if (not (Variables|/Game/Blueprint/BP_ChessTile.BP_ChessTile_C|GethasPiece? (CallFunction|GetTilefromColumnandRow (Variables|/Game/Blueprint/GameInstanceAndLibrary/BP_GameInstance.BP_GameInstance_C|Getchessboard (CallFunction|GetChessInstance)) (Variables|/Game/Blueprint/BP_ChessTile.BP_ChessTile_C|GettileColumn _currenttile_3) _index)))
        (Utilities|Array|Add (Variables|Default|GetpossibleTiles) (CallFunction|GetTilefromColumnandRow (Variables|/Game/Blueprint/GameInstanceAndLibrary/BP_GameInstance.BP_GameInstance_C|Getchessboard (CallFunction|GetChessInstance)) (Variables|/Game/Blueprint/BP_ChessTile.BP_ChessTile_C|GettileColumn _currenttile_3) _index))
        (else
          (Utilities|Array|Add (Variables|Default|GetpossibleTiles) (CallFunction|GetTilefromColumnandRow (Variables|/Game/Blueprint/GameInstanceAndLibrary/BP_GameInstance.BP_GameInstance_C|Getchessboard (CallFunction|GetChessInstance)) (Variables|/Game/Blueprint/BP_ChessTile.BP_ChessTile_C|GettileColumn _currenttile_3) _index))
          (goto _label Break))))
    (:Completed
      (bind _index_2 (Utilities|FlowControl|ForLoopwithBreak (* (Math|Integer|Clamp(Integer) (- _tilerow_2 1) 1 8) -1) (* (Math|Integer|Clamp(Integer) (- _tilerow_2 8) 1 8) -1) :!label _label_2)
        (:LoopBody
          (if (not (Variables|/Game/Blueprint/BP_ChessTile.BP_ChessTile_C|GethasPiece? (CallFunction|GetTilefromColumnandRow (Variables|/Game/Blueprint/GameInstanceAndLibrary/BP_GameInstance.BP_GameInstance_C|Getchessboard (CallFunction|GetChessInstance)) (Variables|/Game/Blueprint/BP_ChessTile.BP_ChessTile_C|GettileColumn _currenttile_4) (Math|Integer|Absolute(Integer) _index_2))))
            (Utilities|Array|Add (Variables|Default|GetpossibleTiles) (CallFunction|GetTilefromColumnandRow (Variables|/Game/Blueprint/GameInstanceAndLibrary/BP_GameInstance.BP_GameInstance_C|Getchessboard (CallFunction|GetChessInstance)) (Variables|/Game/Blueprint/BP_ChessTile.BP_ChessTile_C|GettileColumn _currenttile_4) (Math|Integer|Absolute(Integer) _index_2)))
            (else
              (Utilities|Array|Add (Variables|Default|GetpossibleTiles) (CallFunction|GetTilefromColumnandRow (Variables|/Game/Blueprint/GameInstanceAndLibrary/BP_GameInstance.BP_GameInstance_C|Getchessboard (CallFunction|GetChessInstance)) (Variables|/Game/Blueprint/BP_ChessTile.BP_ChessTile_C|GettileColumn _currenttile_4) (Math|Integer|Absolute(Integer) _index_2)))
              (goto _label_2 Break))))
        (:Completed
          ;[0 0 0 1 36] Calculate Horizontal Moves
          (bind _index_3 (Utilities|FlowControl|ForLoopwithBreak (Math|Integer|Clamp(Integer) (+ _column 1) 0 7) (Math|Integer|Clamp(Integer) (+ _column 8) 0 7) :!label _label_3)
            (:LoopBody
              (if (not (Variables|/Game/Blueprint/BP_ChessTile.BP_ChessTile_C|GethasPiece? (Utilities|Array|Get(acopy) (Utilities|Struct|BreakS_Columns (Utilities|Array|Get(acopy) (Utilities|Struct|BreakS_Rows (Variables|/Game/Blueprint/GameInstanceAndLibrary/BP_GameInstance.BP_GameInstance_C|Getchessboard (CallFunction|GetChessInstance))) (Utilities|Select :Index (Math|Integer|Clamp(Integer) (Variables|/Game/Blueprint/BP_ChessTile.BP_ChessTile_C|GettileRow _currenttile_2) 1 8) :Option%200 0 :Option%201 0 :Option%202 1 :Option%203 2 :Option%204 3 :Option%205 4 :Option%206 5 :Option%207 6 :Option%208 7))) _index_3)))
                (Utilities|Array|Add (Variables|Default|GetpossibleTiles) (Utilities|Array|Get(acopy) (Utilities|Struct|BreakS_Columns (Utilities|Array|Get(acopy) (Utilities|Struct|BreakS_Rows (Variables|/Game/Blueprint/GameInstanceAndLibrary/BP_GameInstance.BP_GameInstance_C|Getchessboard (CallFunction|GetChessInstance))) (Utilities|Select :Index (Math|Integer|Clamp(Integer) (Variables|/Game/Blueprint/BP_ChessTile.BP_ChessTile_C|GettileRow _currenttile_2) 1 8) :Option%200 0 :Option%201 0 :Option%202 1 :Option%203 2 :Option%204 3 :Option%205 4 :Option%206 5 :Option%207 6 :Option%208 7))) _index_3))
                (else
                  (Utilities|Array|Add (Variables|Default|GetpossibleTiles) (Utilities|Array|Get(acopy) (Utilities|Struct|BreakS_Columns (Utilities|Array|Get(acopy) (Utilities|Struct|BreakS_Rows (Variables|/Game/Blueprint/GameInstanceAndLibrary/BP_GameInstance.BP_GameInstance_C|Getchessboard (CallFunction|GetChessInstance))) (Utilities|Select :Index (Math|Integer|Clamp(Integer) (Variables|/Game/Blueprint/BP_ChessTile.BP_ChessTile_C|GettileRow _currenttile_2) 1 8) :Option%200 0 :Option%201 0 :Option%202 1 :Option%203 2 :Option%204 3 :Option%205 4 :Option%206 5 :Option%207 6 :Option%208 7))) _index_3))
                  (goto _label_3 Break))))
            (:Completed
              (bind _index_4 (Utilities|FlowControl|ForLoopwithBreak (* (Math|Integer|Clamp(Integer) (- _column_2 1) 0 7) -1) (* (Math|Integer|Clamp(Integer) (- _column_2 8) 0 7) -1) :!label _label_4)
                (:LoopBody
                  (if (not (Variables|/Game/Blueprint/BP_ChessTile.BP_ChessTile_C|GethasPiece? (Utilities|Array|Get(acopy) (Utilities|Struct|BreakS_Columns (Utilities|Array|Get(acopy) (Utilities|Struct|BreakS_Rows (Variables|/Game/Blueprint/GameInstanceAndLibrary/BP_GameInstance.BP_GameInstance_C|Getchessboard (CallFunction|GetChessInstance))) (Utilities|Select :Index (Math|Integer|Clamp(Integer) (Variables|/Game/Blueprint/BP_ChessTile.BP_ChessTile_C|GettileRow _currenttile) 1 8) :Option%200 0 :Option%201 0 :Option%202 1 :Option%203 2 :Option%204 3 :Option%205 4 :Option%206 5 :Option%207 6 :Option%208 7))) (Math|Integer|Absolute(Integer) _index_4))))
                    (Utilities|Array|Add (Variables|Default|GetpossibleTiles) (Utilities|Array|Get(acopy) (Utilities|Struct|BreakS_Columns (Utilities|Array|Get(acopy) (Utilities|Struct|BreakS_Rows (Variables|/Game/Blueprint/GameInstanceAndLibrary/BP_GameInstance.BP_GameInstance_C|Getchessboard (CallFunction|GetChessInstance))) (Utilities|Select :Index (Math|Integer|Clamp(Integer) (Variables|/Game/Blueprint/BP_ChessTile.BP_ChessTile_C|GettileRow _currenttile) 1 8) :Option%200 0 :Option%201 0 :Option%202 1 :Option%203 2 :Option%204 3 :Option%205 4 :Option%206 5 :Option%207 6 :Option%208 7))) (Math|Integer|Absolute(Integer) _index_4)))
                    (else
                      (Utilities|Array|Add (Variables|Default|GetpossibleTiles) (Utilities|Array|Get(acopy) (Utilities|Struct|BreakS_Columns (Utilities|Array|Get(acopy) (Utilities|Struct|BreakS_Rows (Variables|/Game/Blueprint/GameInstanceAndLibrary/BP_GameInstance.BP_GameInstance_C|Getchessboard (CallFunction|GetChessInstance))) (Utilities|Select :Index (Math|Integer|Clamp(Integer) (Variables|/Game/Blueprint/BP_ChessTile.BP_ChessTile_C|GettileRow _currenttile) 1 8) :Option%200 0 :Option%201 0 :Option%202 1 :Option%203 2 :Option%204 3 :Option%205 4 :Option%206 5 :Option%207 6 :Option%208 7))) (Math|Integer|Absolute(Integer) _index_4)))
                      (goto _label_4 Break))))))))))))
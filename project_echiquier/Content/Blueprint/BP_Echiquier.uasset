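; BP_Echiquier is a chessboard actor that builds its checkered grid of tiles in the Construction Script.
; A single loop over width times height adds each tile as an instance to CaseBlanche or CaseNoire, spaced by TileSize.
; Index parity picks the color, shifted on alternate lines; line math mixes width and height, so it assumes a square board.
; A debug "Hello" prints per tile, and BeginPlay is unused.
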(event EventBeginPlay)

(fn ConstructionScript
  (bind _tilesize (Variables|Chessboard|GettileSize))
  (bind _index (Utilities|FlowControl|ForLoopwithBreak 0 (- (* (Variables|Chessboard|GetchessboardWidth) (Variables|Chessboard|GetchessboardHeight)) 1))
    (:LoopBody
      (Variables|Chessboard|SetcurrentIndex _index)
      (Development|PrintString "Hello")
      (Components|InstancedStaticMesh|AddInstance (select (== (Math|Integer|%(Integer) (select (== (Math|Integer|%(Integer) (/ (Variables|Chessboard|GetcurrentIndex) (Variables|Chessboard|GetchessboardHeight)) 2) 0) (Variables|Chessboard|GetcurrentIndex) (+ (Variables|Chessboard|GetcurrentIndex) 1)) 2) 0) (Variables|Default|GetCaseBlanche) (Variables|Default|GetCaseNoire)) (Math|Transform|MakeTransform (Math|Vector|MakeVector (Math|Conversions|ToFloat(Integer) (* (/ (Variables|Chessboard|GetcurrentIndex) (Variables|Chessboard|GetchessboardWidth)) _tilesize)) (Math|Conversions|ToFloat(Integer) (* (Math|Integer|%(Integer) (Variables|Chessboard|GetcurrentIndex) (Variables|Chessboard|GetchessboardHeight)) _tilesize)) 0.0) "0, 0, 0" "1.000000,1.000000,1.000000") false))))
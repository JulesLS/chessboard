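; Chessboard actor that spawns a grid of BP_ChessTile actors from its root location on BeginPlay.
; Each tile gets a checkered color from index and row parity, plus a column letter and row number that assume an 8x8 board.
; Tiles are stored in a flat array and a per-row structure, through which tile D4 is then looked up and given another material.
; An older instance-based layout script remains but never runs.
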(event EventBeginPlay
  (bind _tilesize (Variables|Chessboard|GettileSize))
  (bind _defaultsceneroot (Variables|Default|GetDefaultSceneRoot))
  (bind _returnvalue (Transformation|GetWorldLocation _defaultsceneroot))
  (bind _index (Utilities|FlowControl|ForLoopwithBreak 0 (- (* (Variables|Chessboard|GetchessboardWidth) (Variables|Chessboard|GetchessboardHeight)) 1))
    (:LoopBody
      (Variables|Chessboard|SetcurrentIndex _index)
      (bind _returnvalue_2 (Game|SpawnActorfromClass "/Game/Blueprint/BP_ChessTile.BP_ChessTile_C" (Math|Transform|MakeTransform (Math|Vector|MakeVector (+ (Math|Conversions|ToFloat(Integer) (* (/ (Variables|Chessboard|GetcurrentIndex) (Variables|Chessboard|GetchessboardWidth)) _tilesize)) (.x _returnvalue)) (+ (Math|Conversions|ToFloat(Integer) (* (Math|Integer|%(Integer) (Variables|Chessboard|GetcurrentIndex) (Variables|Chessboard|GetchessboardHeight)) _tilesize)) (.y _returnvalue)) 0.0) "0, 0, 0" "1.000000,1.000000,1.000000") "Undefined" 0 (select (== (Math|Integer|%(Integer) (select (== (Math|Integer|%(Integer) (/ (Variables|Chessboard|GetcurrentIndex) (Variables|Chessboard|GetchessboardHeight)) 2) 0) (Variables|Chessboard|GetcurrentIndex) (+ (Variables|Chessboard|GetcurrentIndex) 1)) 2) 0) "NewEnumerator1" "NewEnumerator0") (Utilities|Select :Index (Math|Integer|%(Integer) (Variables|Chessboard|GetcurrentIndex) 8) :Option%200 "A" :Option%201 "B" :Option%202 "C" :Option%203 "D" :Option%204 "E" :Option%205 "F" :Option%206 "G" :Option%207 "H") (Utilities|Select :Index (/ (Variables|Chessboard|GetcurrentIndex) 8) :Option%200 1 :Option%201 2 :Option%202 3 :Option%203 4 :Option%204 5 :Option%205 6 :Option%206 7 :Option%207 8) 0))
      (Development|PrintString (Utilities|String|ToString(Integer) (Variables|Chessboard|GetcurrentIndex)))
      (Utilities|Array|Add (Variables|Chessboard|GettilesArray) _returnvalue_2)
      (Utilities|Array|Add (Utilities|Struct|BreakS_Columns (Utilities|Array|Get(acopy) (.findtile (Variables|Chessboard|Getrows)) (/ (Variables|Chessboard|GetcurrentIndex) 8))) _returnvalue_2))
    (:Completed
      (Rendering|Material|SetMaterial (Variables|/Game/Blueprint/BP_ChessTile.BP_ChessTile_C|GettileMesh (CallFunction|GetTilefromColumnandRow (Variables|Chessboard|Getrows) "d" 4)) 0 "/Game/Blueprint/Materials/M_EchiquierMarron.M_EchiquierMarron"))))

(fn ConstructionScript)
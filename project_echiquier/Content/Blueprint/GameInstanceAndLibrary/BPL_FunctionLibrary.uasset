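; Blueprint function library that looks up a tile on an 8x8 board from a lettered column (A–H) and a numbered row.
; GetTileFromColumnAndRow clamps the row to 1–8, converts it to a zero-based index through a Select, then indexes the passed row struct's nested arrays.
; SelectOnName supplies the column index by switching on the letter name.
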(fn GetTilefromColumnandRow
  (params (rowStruct :type S%20Rows%20Structure) (column :type Name) (row :type Integer))
  (return (Utilities|Array|Get(acopy) (Utilities|Struct|BreakS_Columns (Utilities|Array|Get(acopy) (Utilities|Struct|BreakS_Rows rowStruct) (Utilities|Select :Index (Math|Integer|Clamp(Integer) row 1 8) :Option%200 0 :Option%201 0 :Option%202 1 :Option%203 2 :Option%204 3 :Option%205 4 :Option%206 5 :Option%207 6 :Option%208 7))) (CallFunction|SelectonName column))))

(fn SelectonName
  (params (name :type Name))
  (switch name name
    (:a
      (return 0))
    (:b
      (return 1))
    (:c
      (return 2))
    (:d
      (return 3))
    (:e
      (return 4))
    (:f
      (return 5))
    (:g
      (return 6))
    (:h
      (return 7))))
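; BP_ChessTile is a single chessboard square that shows its color and coordinate and reacts to cursor hover.
; The construction script picks the white or black board material from TileColor, prints that color, and sets the text label from TileColumn and TileRow.
; Cursor begin and end events on TileMesh toggle the "hovered" scalar material parameter to drive the hover effect.
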(event OnBeginCursorOver(tileMesh)
  (params (TouchedComponent :type Primitive%20Component%20Object%20Reference))
  (Rendering|Material|SetScalarParameterValueonMaterials (Variables|Default|GettileMesh) "hovered" 1.0))

(event OnEndCursorOver(tileMesh)
  (params (TouchedComponent :type Primitive%20Component%20Object%20Reference))
  (Rendering|Material|SetScalarParameterValueonMaterials (Variables|Default|GettileMesh) "hovered" 0.0))

(fn ConstructionScript
  (bind _tilecolor (Variables|Default|GettileColor))
  (Rendering|Material|SetMaterial (Variables|Default|GettileMesh) 0 (Utilities|Select :Index _tilecolor :NewEnumerator0 "/Game/Blueprint/Materials/M_EchiquierBlanc.M_EchiquierBlanc" :NewEnumerator1 "/Game/Blueprint/Materials/M_EchiquierNoir.M_EchiquierNoir"))
  (Development|PrintString (Utilities|String|EnumtoString _tilecolor))
  (Rendering|Components|TextRender|SetText (Variables|Default|GetTextRender) (Utilities|Text|ToText(Name) (Utilities|String|StringToName (Utilities|String|Append (Utilities|String|ToString(Name) (Variables|Default|GettileColumn)) (Utilities|String|ToString(Integer) (Variables|Default|GettileRow)))))))
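; Blueprint function library with helpers for addressing tiles on an 8x8 board labeled with columns A–H and rows 1–8.
; GetTileFromColumnAndRow maps row and column enums to zero-based indices, then reads the tile from a nested row-and-column struct.
; SelectOnName separately converts a column letter name from A to H into the matching index.
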(fn GetTilefromColumnandRow
  (params (rowStruct :type S%20Rows%20Structure) (columnEnum :type E_Columns%20Enum :default "NewEnumerator0") (rowEnum :type E_Rows%20Enum :default "NewEnumerator0"))
  (return (Utilities|Array|Get(acopy) (Utilities|Struct|BreakS_Columns (Utilities|Array|Get(acopy) (Utilities|Struct|BreakS_Rows rowStruct) (Utilities|Select :Index rowEnum :NewEnumerator0 0 :NewEnumerator1 1 :NewEnumerator2 2 :NewEnumerator3 3 :NewEnumerator4 4 :NewEnumerator5 5 :NewEnumerator6 6 :NewEnumerator7 7))) (Utilities|Select :Index columnEnum :NewEnumerator0 0 :NewEnumerator1 1 :NewEnumerator2 2 :NewEnumerator3 3 :NewEnumerator4 4 :NewEnumerator5 5 :NewEnumerator6 6 :NewEnumerator7 7))))

(fn SelectonName
  (params (name :type Name))
  (switch name name
    (:a
      (return 0))
    (:b
      (return 1))
    (:c
      (return 2))
    (:d
      (return 3))
    (:e
      (return 4))
    (:f
      (return 5))
    (:g
      (return 6))
    (:h
      (return 7))))